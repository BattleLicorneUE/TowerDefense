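; BP_AIMaster is a base AI pawn that walks an ordered waypoint list and can be damaged and destroyed.
; It chains AI MoveTo calls through AllWaypoint, advancing on success or failure until the last index.
; Damage updates the WB_LifeAI widget and shows it temporarily via a retriggerable delay.
; At zero health it spawns a Niagara effect once, removes itself from SpawnAI's array and destroys itself.
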(event Custom|Move%20to%20Next%20Index
  (AI|AIMoveTo self "0, 0, 0" (Utilities|Array|Get(acopy) (Variables|Default|GetAll%20Waypoint) (Variables|Default|GetIndex%20Waypoint)) 5.0 false
    (:OnSuccess
      _)
    (:OnFail
      _))
  (Utilities|FlowControl|Delay 0.1)
  (if (not (== (Utilities|Array|LastIndex (Variables|Default|GetAll%20Waypoint)) (Variables|Default|GetIndex%20Waypoint)))
    (Variables|Default|SetIndex%20Waypoint (+ 1 (Variables|Default|GetIndex%20Waypoint)))
    (CallFunction|MovetoNextIndex)))

(event Custom|Destroy%20AI
  (Default|RemoveAIArray (Variables|Default|GetSpawn%20AI) self)
  (Actor|DestroyActor))

(event EventBeginPlay
  (Utilities|FlowControl|Delay 0.1)
  (CallFunction|MovetoNextIndex)
  (CallFunction|UpdateLife))

(event Game|Damage|EventAnyDamage
  (params (Damage :type Float%20%28single-precision%29) (DamageType :type Damage%20Type%20Object%20Reference) (InstigatedBy :type Controller%20Object%20Reference) (DamageCauser :type Actor%20Object%20Reference))
  (bind _output_get (Variables|Default|SetHealth (- (Variables|Default|GetHealth) Damage)))
  (CallFunction|UpdateLife)
  (if (<= _output_get 0.0)
    (Utilities|FlowControl|DoOnce false
      (:Completed
        (Niagara|SpawnSystematLocation "/Game/VFX/NS_Destroy.NS_Destroy" (Transformation|GetActorLocation self))
        (CallFunction|DestroyAI)))
    (else
      (CallFunction|DisplayLifeBar true)
      (Utilities|FlowControl|RetriggerableDelay 5.0)
      (CallFunction|DisplayLifeBar false))))

(fn ConstructionScript)

(fn UpdateLife
  (bind _aswb_life_ai (Utilities|Casting|CastToWB_LifeAI (UserInterface|GetUserWidgetObject (Variables|Default|GetWidget_Health))))
  (Variables|/Game/Blueprints/HUD/AI/WB_LifeAI.WB_LifeAI_C|SetLife _aswb_life_ai (Math|Float|MapRangeClamped (Variables|Default|GetHealth) 0.0 1e+02 0.0 1.0)))

(fn DisplayLifeBar
  (params (bNewVisibility :type Boolean))
  (Rendering|SetVisibility (Variables|Default|GetWidget_Health) bNewVisibility false))