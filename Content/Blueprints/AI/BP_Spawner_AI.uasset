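; BP_Spawner_AI is a portal spawner that releases one wave of AI pawns on BeginPlay while its portal mesh spins every tick.
; A delayed loop over the NumberAI class array spawns each pawn at the AISpawn component with a Niagara spawn effect.
; Each spawned BP_AIMaster receives the Portal reference and Waypoint data, and the Waves counter increments when the loop completes.
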(event Custom|Spawn%20AI
  (bind _aispawn (Variables|Default|GetAISpawn))
  (bind _aispawn_2 (Variables|Default|GetAISpawn))
  (bind _array_element (Utilities|SpawnAIforDelay (Variables|Default|GetNumber%20AI))
    (:LoopBody
      (bind _returnvalue (AI|SpawnAIFromClass _array_element 0 (Transformation|GetWorldLocation _aispawn_2) (Transformation|GetWorldRotation _aispawn_2) true 0))
      (bind _asbp_aimaster (Utilities|Casting|CastToBP_AIMaster _returnvalue))
      (Variables|/Game/Blueprints/AI/BP_AIMaster.BP_AIMaster_C|SetRef%20Portal _asbp_aimaster (Variables|CustomSettings|GetPortal))
      (Variables|/Game/Blueprints/AI/BP_AIMaster.BP_AIMaster_C|SetAll%20Waypoint _asbp_aimaster (Variables|CustomSettings|GetWaypoint))
      (Niagara|SpawnSystematLocation "/Game/VFX/NS_Spawing.NS_Spawing" (Transformation|GetWorldLocation _aispawn) (Transformation|GetWorldRotation _aispawn)))
    (:Completed
      (Math|Integer|IncrementInt (Variables|Default|GetWaves)))))

(event EventTick
  (params (DeltaSeconds :type Float%20%28single-precision%29))
  (Transformation|AddRelativeRotation (Variables|Default|GetStaticPortal) "0,2.000000, 0" false false))

(event EventBeginPlay
  (CallFunction|SpawnAI))

(fn ConstructionScript)