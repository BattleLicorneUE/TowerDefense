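; BP_Spawner_AI is a portal actor that spawns waves of AI pawns and spins its portal mesh every tick.
; SpawnAI uses a delayed loop to spawn each pawn class at AISpawn with a Niagara effect, tracking it and passing it the spawner, portal and waypoint references.
; RemoveAIArray untracks an AI and, once none remain, tells BP_PlayerController to start the countdown before the next wave.
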(event Custom|Spawn%20AI
  (bind _aispawn (Variables|Default|GetAISpawn))
  (bind _aispawn_2 (Variables|Default|GetAISpawn))
  (bind _array_element (Utilities|SpawnAIforDelay (Variables|Default|GetNumber%20AI))
    (:LoopBody
      (bind _returnvalue (AI|SpawnAIFromClass _array_element 0 (Transformation|GetWorldLocation _aispawn_2) (Transformation|GetWorldRotation _aispawn_2) true 0))
      (bind _asbp_aimaster (Utilities|Casting|CastToBP_AIMaster _returnvalue))
      (Utilities|Array|AddUnique (Variables|Default|GetArray%20AI) _asbp_aimaster)
      (Variables|/Game/Blueprints/AI/BP_AIMaster.BP_AIMaster_C|SetSpawn%20AI _asbp_aimaster self)
      (Variables|/Game/Blueprints/AI/BP_AIMaster.BP_AIMaster_C|SetRef%20Portal _asbp_aimaster (Variables|CustomSettings|GetPortal))
      (Variables|/Game/Blueprints/AI/BP_AIMaster.BP_AIMaster_C|SetAll%20Waypoint _asbp_aimaster (Variables|CustomSettings|GetWaypoint))
      (Niagara|SpawnSystematLocation "/Game/VFX/NS_Spawing.NS_Spawing" (Transformation|GetWorldLocation _aispawn) (Transformation|GetWorldRotation _aispawn)))))

(event Custom|Remove%20AI%20Array
  (params (AIToFind :type BP%20AI%20Master%20Object%20Reference%20%28by%20ref%29))
  (Utilities|Array|RemoveItem (Variables|Default|GetArray%20AI) AIToFind)
  (if (<= (Utilities|Array|Length (Variables|Default|GetArray%20AI)) 0)
    (bind _asbp_player_controller (Utilities|Casting|CastToBP_PlayerController (Game|GetPlayerController 0)))
    (Default|StartTimeBeforeWave _asbp_player_controller)
    (Development|PrintString "Start Waves")
    (else
      (Development|PrintString "Remove"))))

(event EventTick
  (params (DeltaSeconds :type Float%20%28single-precision%29))
  (Transformation|AddRelativeRotation (Variables|Default|GetStaticPortal) "0,2.000000, 0" false false))

(fn ConstructionScript)