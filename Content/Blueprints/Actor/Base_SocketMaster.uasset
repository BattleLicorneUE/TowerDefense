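; Base socket actor that acts as a clickable build spot for towers.
; While empty, its static mesh turns translucent green on cursor hover and back to white when the cursor leaves.
; Clicking an empty socket spawns a Tower_Master at OriginSpawnActor and stores it in RefTower, which disables the highlight and blocks further builds.
; Opening a construction panel is only a debug print.
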(event OnClicked(StaticMesh)
  (params (TouchedComponent :type Primitive%20Component%20Object%20Reference) (ButtonPressed :type Key%20Structure :default "None"))
  (Variables|Default|GetRefTower%20
    (:then
      (Development|PrintString "the tower is already built "))
    (:else
      (Development|PrintString "OpenPanelConstruct")
      (bind _returnvalue (Game|SpawnActorfromClass "/Game/Blueprints/Actor/Tower_Master.Tower_Master_C" (Transformation|GetWorldTransform (Variables|Default|GetOriginSpawnActor)) "Undefined" 0 0))
      (Variables|Default|SetRefTower%20 _returnvalue)
      (Rendering|Material|SetMaterial (Variables|Default|GetStaticMesh) 0 "/Game/Mesh/InstanceMaterials/M_White.M_White"))))

(event OnBeginCursorOver(StaticMesh)
  (params (TouchedComponent :type Primitive%20Component%20Object%20Reference))
  (Variables|Default|GetRefTower%20
    (:then)
    (:else
      (Rendering|Material|SetMaterial (Variables|Default|GetStaticMesh) 0 "/Game/Mesh/InstanceMaterials/M_Opacity_Green.M_Opacity_Green"))))

(event OnEndCursorOver(StaticMesh)
  (params (TouchedComponent :type Primitive%20Component%20Object%20Reference))
  (Variables|Default|GetRefTower%20
    (:then)
    (:else
      (Rendering|Material|SetMaterial (Variables|Default|GetStaticMesh) 0 "/Game/Mesh/InstanceMaterials/M_White.M_White"))))

(fn ConstructionScript)