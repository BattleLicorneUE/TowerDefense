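; Tower_Master is a tower actor, apparently a defense turret, that damages AI pawns.
; Its Sphere overlap stores any entering BP_AIMaster as Target, replacing the previous one and never clearing it.
; A Delay on Tick throttles fire to about five times a second, tracing for Pawns from Target back to OriginShoot.
; The debug-drawn trace ignores the player, and whichever actor it hits takes fixed damage.
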(event OnComponentBeginOverlap(Sphere)
  (params (OverlappedComponent :type Primitive%20Component%20Object%20Reference) (OtherActor :type Actor%20Object%20Reference) (OtherComp :type Primitive%20Component%20Object%20Reference) (OtherBodyIndex :type Integer) (bFromSweep :type Boolean) (SweepResult :type Hit%20Result%20Structure%20%28by%20ref%29))
  (bind _asbp_aimaster (Utilities|Casting|CastToBP_AIMaster OtherActor))
  (Variables|Default|SetTarget _asbp_aimaster))

(event EventTick
  (params (DeltaSeconds :type Float%20%28single-precision%29))
  (Utilities|FlowControl|Delay (/ 1.0 5.0))
  (bind _target (Variables|Default|GetTarget)
    (:then
      (bind (_outhit _returnvalue) (Collision|LineTraceForObjects (Transformation|GetActorLocation _target) (Transformation|GetWorldLocation (Variables|Default|GetOriginShoot)) (Utilities|Array|MakeArray "ObjectTypeQuery3") false (Utilities|Array|MakeArray (Game|GetPlayerCharacter 0)) "ForDuration" true "(R=1.000000,G=0.000000,B=0.000000,A=1.000000)" "(R=0.000000,G=1.000000,B=0.000000,A=1.000000)" 1.0))
      (if _returnvalue
        (Game|Damage|ApplyDamage (.HitActor (Collision|BreakHitResult _outhit)) 5.0 0 0)))
    (:else)))

(fn ConstructionScript)